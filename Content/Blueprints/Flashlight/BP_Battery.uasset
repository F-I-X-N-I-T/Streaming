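; BP_Battery is a battery pickup for the flashlight system, collected by pressing F inside its Box trigger.
; Box overlap begin and end toggle the actor's input from player controller 0.
; On F, it messages the overlapping actor to add a battery, then queries its inventory for a flashlight.
; Either result prints a placeholder Spanish message marked for a later widget change, and the battery destroys itself.
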(event `Key|F`
  (params (Key :type "Key Structure"))
  (:`Pressed`
    (message `/Game/Blueprints/Interfaces/BPI_Inventory.Add_Battery` (stale `self.Box.OnComponentBeginOverlap` OtherActor) "")
    (bind _flashlight_ (message `/Game/Blueprints/Interfaces/BPI_Inventory.Check_Inventory` (stale `self.Box.OnComponentBeginOverlap` OtherActor) "" ""))
    (if _flashlight_
      (`KismetSystemLibrary.PrintString` "\"La linterna tiene energia o asi xd\" Y CAMBIAR ESTO EN EL WIDGET")
      (else
        (`KismetSystemLibrary.PrintString` "\"Necesitas una linterna\" Y CAMBIAR ESTO EN EL WIDGET")))
    (`self.K2_DestroyActor`)))

(event `self.Box.OnComponentBeginOverlap`
  (params (OverlappedComponent :type "PrimitiveComponent Object Reference") (OtherActor :type "Actor Object Reference") (OtherComp :type "PrimitiveComponent Object Reference") (OtherBodyIndex :type Integer) (bFromSweep :type Boolean) (SweepResult :type "HitResult Structure (by ref)"))
  (`self.EnableInput` (`GameplayStatics.GetPlayerController` 0)))

(event `self.Box.OnComponentEndOverlap`
  (params (OverlappedComponent :type "PrimitiveComponent Object Reference") (OtherActor :type "Actor Object Reference") (OtherComp :type "PrimitiveComponent Object Reference") (OtherBodyIndex :type Integer))
  (`self.DisableInput` (`GameplayStatics.GetPlayerController` 0)))

(fn `UserConstructionScript`)